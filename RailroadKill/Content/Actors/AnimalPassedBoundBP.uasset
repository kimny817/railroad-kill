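; AnimalPassedBoundBP is a boundary actor that counts passing animals to decide when the level is passed.
; It adds a ScoreUI widget at BeginPlay, then increments and prints TotalAnimalsPassed on every overlap, without filtering the other actor.
; Once the count reaches LevelPassedCount, it shows LevelPassedDisplay and starts a timer that opens Level_Scene after a short delay.
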(event `self.ReceiveBeginPlay`
  (bind _returnvalue (`|CreateWidget` "/Game/Actors/ScoreUI.ScoreUI_C"))
  (`UserWidget.AddToViewport` _returnvalue 0))

(event `self.ReceiveActorBeginOverlap`
  (params (OtherActor :type "Actor Object Reference"))
  (bind _totalanimalspassed (`self.TotalAnimalsPassed`))
  (bind _result (`/Engine/EditorBlueprintResources/StandardMacros.IncrementInt` _totalanimalspassed)
    (:`  `
      (`KismetSystemLibrary.PrintString` (`KismetStringLibrary.Conv_IntToString` _result))
      (if (>= _totalanimalspassed (`self.LevelPassedCount`))
        (`KismetSystemLibrary.K2_SetTimer` null "LevelPassedFn" 2.0)
        (bind _returnvalue (`|CreateWidget` "/Game/Actors/LevelPassedDisplay.LevelPassedDisplay_C"))
        (`UserWidget.AddToViewport` _returnvalue 0)))))

(fn `LevelPassedFn`
  (`GameplayStatics.OpenLevel` "Level_Scene"))

(fn `UserConstructionScript`)