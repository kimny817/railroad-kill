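; FollowTrainBP is a train car actor that trails a parent train along its spline.
; Only the first car updates on Tick, placing itself at the parent's spline Alpha minus an Offset, using a valid fork train or otherwise the stop train.
; Each car then recursively positions the next car in the linked chain, doubling the passed Offset at every step.
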(event `self.ReceiveTick`
  (params (DeltaSeconds :type "Float (single-precision)"))
  (if (`self.IsFirst`)
    (`self.Update LocationRotation` (`self.Offset`))))

(fn `Update LocationRotation`
  (params (Offset :type "Float (double-precision)"))
  (bind _nexttraincar (`self.NextTrainCar`))
  (bind _parentforktrain (`self.ParentForkTrain`))
  (bind _parentstoptrain (`self.ParentStopTrain`))
  (if (`KismetSystemLibrary.IsValid` _parentforktrain)
    (bind (_position _rotation) (`/Game/Actors/ForkTrainBP.GetSplinePositionRotation` _parentforktrain (- (`/Game/Actors/ForkTrainBP.Alpha` _parentforktrain) Offset)))
    (`self.K2_SetActorLocationAndRotation` _position _rotation)
    (else
      (bind (_position_2 _rotation_2) (`/Game/Actors/StopTrainBP.GetSplinePositionRotation` _parentstoptrain (- (`/Game/Actors/StopTrainBP.Alpha` _parentstoptrain) Offset)))
      (`self.K2_SetActorLocationAndRotation` _position_2 _rotation_2)))
  (if (`KismetSystemLibrary.IsValid` _nexttraincar)
    (`self.Update LocationRotation` _nexttraincar (+ Offset (`self.Offset`)))))

(fn `UserConstructionScript`)