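; Train actor that rides one of two railroad splines and can switch between them.
; On BeginPlay, if active, a timeline scaled by duration and start offset moves it along the current railroad by distance, matching position and rotation.
; Toggle and setter functions swap the current railroad, which the movement reads each update.
; Clicking the train mesh plays an explosion sound and calls StartPause on all Animal actors.
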(event `self.ReceiveBeginPlay`
  (if (`self.ActiveTrain`)
    (`self.MoveTrain`)))

(event `MoveTrain`
  (`TimelineComponent.SetPlayRate` (`self.TrainMover`) (/ 1.0 (`self.Duration`)))
  (`TimelineComponent.SetNewTime` (`self.TrainMover`) (`self.StartOffset `))
  (bind (_direction _alpha) (`Timeline|TrainMover`)
    (:`Update`
      (bind _output_get (set `self.Alpha` _alpha))
      (bind (_position _rotation) (`self.GetSplinePositionRotation` _output_get))
      (`self.K2_SetActorLocationAndRotation` _position _rotation))))

(event `self.TrainMesh.OnClicked`
  (params (TouchedComponent :type "PrimitiveComponent Object Reference") (ButtonPressed :type "Key Structure"))
  (`GameplayStatics.PlaySoundAtLocation` "/Game/StarterContent/Audio/Explosion01.Explosion01" (`self.K2_GetActorLocation`) (struct) 1.0 1.0 0.0 null null null)
  (bind _outactors (`GameplayStatics.GetAllActorsOfClass` "/Game/Actors/Animal.Animal_C"))
  (for _array_element _outactors
    (`/Game/Actors/Animal.StartPause` _array_element)))

(event `/Game/Actors/TrainInterface.ToggleTrainMode`
  (if (== (`self.RailroadCurrent`) (`self.Railroad1`))
    (set `self.RailroadCurrent` (`self.Railroad2`))
    (else
      (set `self.RailroadCurrent` (`self.Railroad1`)))))

(fn `GetSplinePositionRotation`
  (params (T :type "Float (double-precision)"))
  (returns (Position :type "Vector Structure") (Rotation :type "Rotator Structure"))
  (bind _railroadcurrent (`self.RailroadCurrent`))
  (bind _returnvalue (`KismetMathLibrary.Lerp` 0.0 (`SplineComponent.GetSplineLength` (`/Game/Actors/RailroadBP.Spline` _railroadcurrent)) T))
  (return (`SplineComponent.GetLocationAtDistanceAlongSpline` (`/Game/Actors/RailroadBP.Spline` _railroadcurrent) _returnvalue "World") (`SplineComponent.GetRotationAtDistanceAlongSpline` (`/Game/Actors/RailroadBP.Spline` _railroadcurrent) _returnvalue "World")))

(fn `SwitchRailroads`
  (params (NewParam :type "/Game/Actors/RailroadBP Object Reference"))
  (set `self.RailroadCurrent` NewParam))

(fn `UserConstructionScript`
  (set `self.RailroadCurrent` (`self.Railroad1`)))