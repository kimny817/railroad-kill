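; StopTrainBP is a train actor that travels along the spline of a referenced railroad and can make timed stops.
; A timeline, rate-scaled by Duration, drives an alpha that maps to distance along the spline for world location and rotation, starting on BeginPlay if ActiveTrain.
; ToggleTrainMode pauses it for a short fixed delay, then resumes from the saved AlphaPrime.
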(event `self.ReceiveBeginPlay`
  (if (`self.ActiveTrain`)
    (`self.MoveTrain`)))

(event `MoveTrain`
  (`TimelineComponent.SetPlayRate` (`self.TrainMover`) (/ 1.0 (`self.Duration`)))
  (`TimelineComponent.SetNewTime` (`self.TrainMover`) (`self.Alpha_Prime`))
  (bind (_direction _alpha) (`Timeline|TrainMover` :!label _label)
    (:`Update`
      (bind _output_get (set `self.Alpha` _alpha))
      (if (`self.Paused`)
        (goto _label :!via `Stop`)
        (else
          (set `self.Alpha_Prime` _output_get)
          (bind (_position _rotation) (`self.GetSplinePositionRotation` _output_get))
          (`self.K2_SetActorLocationAndRotation` _position _rotation))))))

(event `/Game/Actors/TrainInterface.ToggleTrainMode`
  (set `self.Paused` true)
  (`KismetSystemLibrary.Delay` 2.0)
  (set `self.Paused` false)
  (`self.MoveTrain`))

(fn `GetSplinePositionRotation`
  (params (T :type "Float (double-precision)"))
  (returns (Position :type "Vector Structure") (Rotation :type "Rotator Structure"))
  (bind _returnvalue (`KismetMathLibrary.Lerp` 0.0 (`SplineComponent.GetSplineLength` (`/Game/Actors/RailroadBP.Spline` (`self.Railroad1`))) T))
  (return (`SplineComponent.GetLocationAtDistanceAlongSpline` (`/Game/Actors/RailroadBP.Spline` (`self.Railroad1`)) _returnvalue "World") (`SplineComponent.GetRotationAtDistanceAlongSpline` (`/Game/Actors/RailroadBP.Spline` (`self.Railroad1`)) _returnvalue "World")))

(fn `UserConstructionScript`)