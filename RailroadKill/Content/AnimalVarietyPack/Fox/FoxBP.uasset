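; Fox obstacle actor that runs along world Y at a constant speed and triggers game over on contact.
; Tick moves it by a speed set on BeginPlay, scaled by delta time.
; Any overlap with an actor not named with the "AnimalPassed" prefix shows the game-over widget, spawns kill particles and explosion audio, and sets a delayed timer for "Gameover", a function not defined here.
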(event `self.ReceiveActorBeginOverlap`
  (params (OtherActor :type "Actor Object Reference"))
  (bind _returnvalue (`self.K2_GetActorLocation`))
  (if (not (`KismetStringLibrary.StartsWith` (`KismetSystemLibrary.GetDisplayName` OtherActor) "AnimalPassed"))
    (`KismetSystemLibrary.K2_SetTimer` null "Gameover" 2.0)
    (bind _returnvalue_2 (`|CreateWidget` "/Game/GameOverDisplay.GameOverDisplay_C"))
    (`UserWidget.AddToViewport` _returnvalue_2 0)
    (`|SpawnActorFromClass` "/Game/AnimalKillParticles.AnimalKillParticles_C" (`KismetMathLibrary.MakeTransform` _returnvalue) "Undefined" "OverrideRootScale" null null)
    (`GameplayStatics.PlaySoundAtLocation` "/Game/StarterContent/Audio/Explosion02.Explosion02" _returnvalue (struct) 0.3 0.5 0.0 null null null)))

(event `self.ReceiveBeginPlay`
  (bind _output_get (set `self.Speed` 400.0)))

(event `self.ReceiveTick`
  (params (DeltaSeconds :type "Float (single-precision)"))
  (`self.K2_SetActorLocationAndRotation` (+ (`self.K2_GetActorLocation`) (`KismetMathLibrary.MakeVector` 0.0 (* (stale `self.ReceiveBeginPlay` _output_get) (`GameplayStatics.GetWorldDeltaSeconds`))))))

(fn `UserConstructionScript`)