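; Train actor that rides along the spline of a referenced railroad actor when flagged active.
; On BeginPlay it starts a timeline whose play rate comes from a duration and whose start time comes from an offset.
; Each update maps the timeline alpha to a distance along the spline and sets the train's world location and rotation to match.
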(event `self.ReceiveBeginPlay`
  (if (`self.ActiveTrain`)
    (`self.MoveTrain`)))

(event `MoveTrain`
  (bind _returnvalue (`KismetMathLibrary.Lerp` 0.0 (`SplineComponent.GetSplineLength` (`/Game/RailroadBP.Spline` (`self.RailroadRef`))) (`self.Alpha`)))
  (`TimelineComponent.SetPlayRate` (`self.TrainMover`) (/ 1.0 (`self.Duration`)))
  (`TimelineComponent.SetNewTime` (`self.TrainMover`) (`self.StartOffset `))
  (bind (_direction _alpha) (`Timeline|TrainMover`)
    (:`Update`
      (set `self.Alpha` _alpha)
      (`self.K2_SetActorLocationAndRotation` (`SplineComponent.GetLocationAtDistanceAlongSpline` (`/Game/RailroadBP.Spline` (`self.RailroadRef`)) _returnvalue "World") (`SplineComponent.GetRotationAtDistanceAlongSpline` (`/Game/RailroadBP.Spline` (`self.RailroadRef`)) _returnvalue "World")))))

(fn `UserConstructionScript`)